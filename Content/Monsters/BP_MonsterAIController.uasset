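; AI controller for a monster that chases the main hero on sight.
; On BeginPlay it binds OnSee to the pawn's PawnSensing component, which caches the hero and issues a move to the hero's current location.
; While the seen flag is clear, Tick re-checks line of sight to the cached hero, re-runs OnSee and turns the pawn along control rotation.
; A MoveTo actor helper is defined but not called here.
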(event `self.ReceiveTick`
  (params (DeltaSeconds :type "Float (single-precision)"))
  (if (== (`self.IsPlayerSeen`) false)
    (if (== (`self.LineOfSightTo` (stale `OnSee` _asbp_main_hero_mesh)) true)
      (`self.OnSee` (stale `OnSee` _asbp_main_hero_mesh))
      (`self.K2_SetActorRotation` (`self.K2_GetPawn`) (`KismetMathLibrary.MakeRotFromX` (`KismetMathLibrary.GetForwardVector` (`self.GetControlRotation`))) false))))

(event `self.ReceiveBeginPlay`
  (add `PawnSensingComponent.OnSeePawn` (`self.GetComponentByClass` (`self.K2_GetPawn`) "/Script/AIModule.PawnSensingComponent") (delegate `OnSee`)))

(event `OnSee`
  (params (Pawn :type "Pawn Object Reference"))
  (set `self.IsPlayerSeen` true)
  (`KismetSystemLibrary.PrintString` "Seen")
  (bind _asbp_main_hero_mesh (cast `/Game/MainHero/BP_MainHeroMesh` Pawn))
  (`self.MoveToLocation` (`self.K2_GetActorLocation` _asbp_main_hero_mesh) -1.0 true true false true null)
  (set `self.IsPlayerSeen` false))

(fn `MoveTo`
  (params (Target :type "/Game/MainHero/BP_MainHeroMesh Object Reference"))
  (`self.MoveToActor` Target -1.0 true true true null))

(fn `UserConstructionScript`)