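; AI controller for a flying monster that chases the main hero.
; On BeginPlay it binds the pawn's PawnSensing to OnSee, which casts the seen pawn to the hero, caches it and calls MoveToActor.
; Tick turns the monster along its control rotation while the cached hero is in line of sight.
; Tick's damage and sight checks re-call OnSee with the controlled pawn, not the hero, so that cast gates any re-chase.
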(event `self.ReceiveTick`
  (params (DeltaSeconds :type "Float (single-precision)"))
  (bind _returnvalue (`self.K2_GetPawn`))
  (`|ExecutionSequence`
    (:`then_0`
      (bind _asentity (cast `Entity` _returnvalue))
      (bind _returnvalue_2 (`Entity.getBeingDamaged` _asentity))
      (if _returnvalue_2
        (`self.OnSee` _returnvalue)))
    (:`then_1`
      (if (== (`self.LineOfSightTo` (stale `OnSee` _asbp_main_hero_mesh)) true)
        (`self.OnSee` _returnvalue)
        (`self.K2_SetActorRotation` _returnvalue (`KismetMathLibrary.MakeRotFromX` (`KismetMathLibrary.GetForwardVector` (`self.GetControlRotation`))) false)))))

(event `self.ReceiveBeginPlay`
  (add `PawnSensingComponent.OnSeePawn` (`self.GetComponentByClass` (`self.K2_GetPawn`) "/Script/AIModule.PawnSensingComponent") (delegate `OnSee`)))

(event `OnSee`
  (params (Pawn :type "Pawn Object Reference"))
  (bind _asbp_main_hero_mesh (cast `/Game/MainHero/BP_MainHeroMesh` Pawn))
  (`self.MoveToActor` _asbp_main_hero_mesh -1.0 true true true null))

(fn `UserConstructionScript`)